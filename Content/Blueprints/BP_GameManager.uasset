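; Game manager Blueprint that holds the money, countdown timer, creature spawn data and upgrade data, and creates the game UI.
; On BeginPlay it finds the player, fills maps from the creature and upgrade data tables, and marks every creature uncollected.
; AddSpawnWeight adjusts a creature's clamped spawn weight, optionally offsetting its "nothing" weight.
; It also toggles player movement, updates the money text and only prints game over at timer expiry.
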(event `self.ReceiveBeginPlay`
  (`|ExecutionSequence`
    (:`then_0`
      (bind _returnvalue (`GameplayStatics.GetActorOfClass` "/Game/TopDown/Blueprints/BP_TopDownCharacter.BP_TopDownCharacter_C"))
      (set `self.playerRef` _returnvalue))
    (:`then_1`
      (`self.InitCreatureSpawns`)
      (`self.InitUpgrades`))
    (:`then_2`
      (bind _returnvalue_2 (`|CreateWidget` "/Game/Blueprints/UI/WB_GameUI.WB_GameUI_C"))
      (`UserWidget.AddToViewport` _returnvalue_2 0)
      (set `self.gameUI` _returnvalue_2)
      (`self.UpdateMoney` 0.0))
    (:`then_3`
      (`self.UpdateMoney` 0.0))))

(event `self.ReceiveTick`
  (params (DeltaSeconds :type "Float (single-precision)"))
  (`self.UpdateTimer`))

(fn `AddSpawnWeight`
  (params (creatureType :type "/Game/Blueprints/Enums/CreatureType Enum" :default "NewEnumerator0") (addAmount :type "Float (double-precision)") (conservePopulation :type Boolean))
  (returns (newWeight :type "Float (double-precision)"))
  (locals (ChangeAmount :type "Float (double-precision)") (originalWeight :type "Float (double-precision)") (minimumWeight :type "Float (double-precision)" :default 1.0) (newNothingWeight :type "Float (double-precision)"))
  (bind _creaturespawns (`self.creatureSpawns`))
  (bind (_value _returnvalue) (`BlueprintMapLibrary.Map_Find` _creaturespawns creatureType))
  (bind (_id _displayname _rarity _value_2 _firsttimebonus _spawnweight _nothingweight) (break `/Game/Blueprints/Data/CreatureData` _value))
  (set `local.ChangeAmount` addAmount)
  ;[1 1 1] Decrease Creature Spawn Weighting
  (`|ExecutionSequence`
    (:`then_0`
      (if _returnvalue
        (bind _output_get (set `local.originalWeight` _spawnweight))
        (bind _returnvalue_2 (`KismetMathLibrary.FMax` (+ _output_get addAmount) (`local.minimumWeight`)))
        (set `local.ChangeAmount` (- _returnvalue_2 _output_get))
        (if conservePopulation
          (bind _output_get_2 (set `local.newNothingWeight` (`KismetMathLibrary.FMax` (- _nothingweight (`local.ChangeAmount`)))))
          (`KismetSystemLibrary.PrintString` (`KismetStringLibrary.Concat_StrStr` "Nothing Weighting:" (`KismetStringLibrary.Conv_DoubleToString` _output_get_2))))
        (bind _structout (setmembers `/Game/Blueprints/Data/CreatureData` :`StructRef` _value :`spawnWeight` _returnvalue_2 :`nothingWeight` (`local.newNothingWeight`)))
        (`BlueprintMapLibrary.Map_Add` _creaturespawns _id _structout)
        (`KismetSystemLibrary.PrintString` (`KismetStringLibrary.Concat_StrStr` (`|GetEnumeratorNameAsString` creatureType) " weighting: " (`KismetStringLibrary.Conv_DoubleToString` _returnvalue_2)))))
    (:`then_2`
      ;[1 1 1] Fill in Spawn Weighting Gap
      (return _returnvalue_2))))

(fn `CanMove`
  (returns (CanMove :type Boolean))
  ;[1 1 1] player can move
  (return (`|EnumInequality` (`CharacterMovementComponent.MovementMode` (`Character.CharacterMovement` (`self.playerRef`))) "MOVE_None")))

(fn `InitCreatureSpawns`
  (`BlueprintMapLibrary.Map_Clear` (`self.creatureSpawns`))
  (`BlueprintMapLibrary.Map_Clear` (`self.collectedCreatures`))
  (bind _outrownames (`DataTableFunctionLibrary.GetDataTableRowNames` "/Game/Blueprints/Data/CreatureSpawnTable.CreatureSpawnTable"))
  (for _array_element _outrownames
    (bind _returnvalue (`|GetDataTableRow` "/Game/Blueprints/Data/CreatureSpawnTable.CreatureSpawnTable" _array_element)
      (:`then`
        (bind _id (break `/Game/Blueprints/Data/CreatureData` _returnvalue))
        (`BlueprintMapLibrary.Map_Add` (`self.creatureSpawns`) _id _returnvalue)
        (`BlueprintMapLibrary.Map_Add` (`self.collectedCreatures`) _id)))))

(fn `InitUpgrades`
  (bind _upgradesdata (`self.upgradesData`))
  (`BlueprintMapLibrary.Map_Clear` _upgradesdata)
  (bind _outrownames (`DataTableFunctionLibrary.GetDataTableRowNames` "/Game/Blueprints/Data/UpgradeTable.UpgradeTable"))
  (for _array_element _outrownames
    (bind _returnvalue (`|GetDataTableRow` "/Game/Blueprints/Data/UpgradeTable.UpgradeTable" _array_element)
      (:`then`
        (`BlueprintMapLibrary.Map_Add` _upgradesdata (`.type_3_31B2B27447C86FD58B71CD9FABF2FE69` (break `/Game/Blueprints/Data/UpgradeData` _returnvalue)) _returnvalue)))))

(fn `SetPlayerMovement`
  (params (canMove :type Boolean))
  (bind _charactermovement (`Character.CharacterMovement` (`self.playerRef`)))
  (if canMove
    (`CharacterMovementComponent.SetMovementMode` _charactermovement "MOVE_Walking" 0)
    (else
      (`CharacterMovementComponent.DisableMovement` _charactermovement))))

(fn `UpdateMoney`
  (params (`added money` :type "Float (double-precision)"))
  (returns (endMoney :type "Float (double-precision)"))
  (bind _output_get (set `self.money` (+ `added money` (`self.money`))))
  (set `TextBlock.Text` (`KismetTextLibrary.Conv_StringToText` (`KismetStringLibrary.Concat_StrStr` "$" (`KismetStringLibrary.Conv_Int64ToString` (`KismetMathLibrary.Round64` _output_get)))) (`/Game/Blueprints/UI/WB_GameUI.moneyText` (`self.gameUI`)))
  (return _output_get))

(fn `UpdateTimer`
  (bind _output_get (set `self.gameTimer` (- (`self.gameTimer`) (`GameplayStatics.GetWorldDeltaSeconds`))))
  (if (<= _output_get 0.0)
    (`KismetSystemLibrary.PrintString` "game over!")))

(fn `UserConstructionScript`)