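; Spawn point actor that spawns a weighted-random BP_Creature at its transform when its Area is unlocked in BP_GameManager.
; SpawnCreature filters the manager's CreatureSpawns by SpawnableCreatures plus a "nothing" entry, then picks by cumulative weight, adjusted per creature by SpawnWeightInfluence.
; The chosen entry initializes the new creature.
; It spawns one tick after BeginPlay, and Tick counts down RespawnTimer to retry whenever no valid creature exists.
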(event `self.ReceiveBeginPlay`
  (bind _returnvalue (`GameplayStatics.GetActorOfClass` "/Game/Blueprints/BP_GameManager.BP_GameManager_C"))
  (set `self.gameManager` _returnvalue)
  (set `self.respawnTimer` (`self.respawnDuration`))
  (`SceneComponent.SetVisibility` (`self.SkeletalMesh`) false false)
  (`KismetSystemLibrary.DelayUntilNextTick`)
  (`self.SpawnCreature`))

(event `self.ReceiveTick`
  (params (DeltaSeconds :type "Float (single-precision)"))
  (`self.UpdateRespawnTimer`))

(fn `SpawnCreature`
  (locals (totalSpawnWeight :type "Float (double-precision)") (currentSpawnWeight :type "Float (double-precision)") (randomWeight :type "Float (double-precision)") (spawnedCreature :type "/Game/Blueprints/Enums/CreatureType Enum"))
  (if (`BlueprintMapLibrary.Map_Find` (`/Game/Blueprints/BP_GameManager.areasUnlocked` (`self.gameManager`)) (`self.area`))
    (set `self.respawnTimer` (`self.respawnDuration`))
    (bind _returnvalue (`GameplayStatics.GetActorOfClass` "/Game/Blueprints/BP_GameManager.BP_GameManager_C"))
    (bind _values (`BlueprintMapLibrary.Map_Values` (`/Game/Blueprints/BP_GameManager.creatureSpawns` _returnvalue)))
    (`|ExecutionSequence`
      (:`then_0`
        (for _array_element _values
          (bind (_id _displayname _rarity _description _value _firsttimebonus _spawnweight _nothingweight) (break `/Game/Blueprints/Data/CreatureData` _array_element))
          (if (or (`|EnumEquality` _id "NewEnumerator2") (>= (`KismetArrayLibrary.Array_Find` (`self.spawnableCreatures`) _id) 0))
            (set `local.totalSpawnWeight` (+ (`local.totalSpawnWeight`) _spawnweight _nothingweight)))))
      (:`then_1`
        ;[1 1 1] Choose a creature from the spawn weight
        (set `local.randomWeight` (`KismetMathLibrary.RandomFloatInRange` 0.0 (`local.totalSpawnWeight`)))
        (for _array_element_2 _values
          (bind (_id_2 _displayname_2 _rarity_2 _description_2 _value_2 _firsttimebonus_2 _spawnweight_2) (break `/Game/Blueprints/Data/CreatureData` _array_element_2))
          (if (or (`|EnumEquality` _id_2 "NewEnumerator2") (>= (`KismetArrayLibrary.Array_Find` (`self.spawnableCreatures`) _id_2) 0))
            (bind _output_get (set `local.currentSpawnWeight` (+ _spawnweight_2 (`local.currentSpawnWeight`))))
            (if (<= (`local.randomWeight`) (+ (`BlueprintMapLibrary.Map_Find` (`self.spawnWeightInfluence`) _id_2) _output_get))
              (if (`|EnumInequality` _id_2 "NewEnumerator2")
                (bind _returnvalue_2 (`|SpawnActorFromClass` "/Game/Blueprints/BP_Creature.BP_Creature_C" (`self.GetTransform`) "Undefined" "MultiplyWithRoot" null null))
                (bind _output_get_2 (set `self.currentCreature` _returnvalue_2))
                (`self.K2_SetActorRotation` _output_get_2 (`SceneComponent.K2_GetComponentRotation` (`self.DefaultSceneRoot`)) false)
                (`/Game/Blueprints/BP_Creature.Initialize Creature` _output_get_2 _array_element_2)
                (break)
                (else
                  (break))))))
        (if (`KismetSystemLibrary.IsValid` (`self.currentCreature`))
          _)))))

(fn `UpdateRespawnTimer`
  (bind _respawntimer (`self.respawnTimer`))
  (`/Engine/EditorBlueprintResources/StandardMacros.IsValid` (`self.currentCreature`)
    (:`Is Not Valid`
      (if (> _respawntimer 0.0)
        (bind _output_get (set `self.respawnTimer` (- _respawntimer (`GameplayStatics.GetWorldDeltaSeconds`))))
        (if (<= _output_get 0.0)
          (`self.SpawnCreature`))))))

(fn `UserConstructionScript`)