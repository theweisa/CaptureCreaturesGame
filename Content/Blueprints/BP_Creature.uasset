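; Creature actor that the player can select, then collect or release, and that despawns when its timer runs out.
; Registers cursor hover with BP_GameManager and each tick checks whether it is selected and within the player's interact range, opening WB_CollectButtons once.
; Collecting lowers its type's spawn weight, releasing applies WeightOnRelease, both conserving population.
; Either action grants a first-time bonus for uncollected types, then destroys the actor.
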(event `self.ReceiveBeginPlay`
  (bind _returnvalue (`GameplayStatics.GetActorOfClass` "/Game/Blueprints/BP_GameManager.BP_GameManager_C"))
  (set `self.gameManager` _returnvalue))

(event `self.ReceiveTick`
  (params (DeltaSeconds :type "Float (single-precision)"))
  (`|ExecutionSequence`
    (:`then_0`
      (`self.CheckInteracted`)
      (if (`self.interacted`)
        _))
    (:`then_1`
      (`self.UpdateDespawnTimer`))))

(event `self.ReceiveActorBeginCursorOver`
  (set `/Game/Blueprints/BP_GameManager.hoveredCreature` self (`self.gameManager`)))

(event `self.ReceiveActorEndCursorOver`
  (bind _gamemanager (`self.gameManager`))
  (if (== (`/Game/Blueprints/BP_GameManager.hoveredCreature` _gamemanager) self)
    (set `/Game/Blueprints/BP_GameManager.hoveredCreature` null _gamemanager)))

(fn `CheckFirstTimeBonus`
  (bind _gamemanager (`self.gameManager`))
  (bind _firsttimebonus (`self.firstTimeBonus`))
  (bind _id (`self.id`))
  (bind _collectedcreatures (`/Game/Blueprints/BP_GameManager.collectedCreatures` _gamemanager))
  (if (not (`BlueprintMapLibrary.Map_Find` _collectedcreatures _id))
    (`/Game/Blueprints/BP_GameManager.UpdateMoney` _gamemanager _firsttimebonus)
    (`KismetSystemLibrary.PrintString` (`KismetStringLibrary.Concat_StrStr` "Bonus Money: " (`KismetStringLibrary.Conv_DoubleToString` _firsttimebonus)))
    (`BlueprintMapLibrary.Map_Add` _collectedcreatures _id true)))

(fn `CheckInteracted`
  (bind _playerref (`/Game/Blueprints/BP_GameManager.playerRef` (`self.gameManager`)))
  (if (and (== (`/Game/Blueprints/BP_GameManager.selectedCreature` (`self.gameManager`)) self) (<= (`self.GetDistanceTo` _playerref self) (`/Game/TopDown/Blueprints/BP_TopDownCharacter.interactDistance` _playerref)) (not (`self.interacted`)) (`|EnumInequality` (`CharacterMovementComponent.MovementMode` (`Character.CharacterMovement` _playerref)) "MOVE_None"))
    (set `self.interacted` true)
    (bind _returnvalue (`|CreateWidget` "/Game/Blueprints/UI/WB_CollectButtons.WB_CollectButtons_C"))
    (`/Game/Blueprints/UI/WB_CollectButtons.InitCollectScreen` _returnvalue self)))

(fn `CollectCreature`
  (bind _gamemanager (`self.gameManager`))
  (`|ExecutionSequence`
    (:`then_0`
      (`/Game/Blueprints/BP_GameManager.AddSpawnWeight` _gamemanager (`self.id`) -1.0 true))
    (:`then_1`
      (`self.CheckFirstTimeBonus`)
      (`/Game/Blueprints/BP_GameManager.UpdateMoney` _gamemanager 0.0))
    (:`then_2`
      (`self.K2_DestroyActor`))))

(fn `InitializeCreature`
  (params (creatureStats :type "/Game/Blueprints/Data/CreatureData Structure"))
  (bind (_id _displayname _rarity _value _firsttimebonus _spawnweight _nothingweight _despawntimer) (break `/Game/Blueprints/Data/CreatureData` creatureStats))
  (`|ExecutionSequence`
    (:`then_0`
      (set `self.id` _id))
    (:`then_1`
      (set `self.rarity` _rarity))
    (:`then_2`
      (set `self.value` _value))
    (:`then_3`
      (`KismetSystemLibrary.PrintString` (`KismetStringLibrary.Concat_StrStr` (`|GetEnumeratorNameAsString` (`self.id`)) ": creature initialized")))
    (:`then_4`
      (set `self.firstTimeBonus` _firsttimebonus))
    (:`then_5`
      (set `self.despawnTimer` _despawntimer))))

(fn `ReleaseCreature`
  (`|ExecutionSequence`
    (:`then_0`
      (`/Game/Blueprints/BP_GameManager.AddSpawnWeight` (`self.gameManager`) (`self.id`) (`self.weightOnRelease`) true))
    (:`then_1`
      (`self.CheckFirstTimeBonus`))
    (:`then_2`
      (`self.K2_DestroyActor`))))

(fn `UpdateDespawnTimer`
  (bind _output_get (set `self.despawnTimer` (- (`self.despawnTimer`) (`GameplayStatics.GetWorldDeltaSeconds`))))
  (if (<= _output_get 0.0)
    (`self.K2_DestroyActor`)))

(fn `UserConstructionScript`)