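; BP_Destructable is a clickable world object that opens a WB_Destructable widget when the player interacts with it.
; Hovering toggles custom depth on its mesh for highlighting, and the highlight stays on once interacted.
; A click checks distance against the player's InteractDistance through BP_GameManager's PlayerRef, requiring active movement and no prior interaction.
; It then disables player movement, sets Interacted and passes itself to the widget.
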(event `self.ReceiveBeginPlay`
  (bind _returnvalue (`GameplayStatics.GetActorOfClass` "/Game/Blueprints/BP_GameManager.BP_GameManager_C"))
  (set `self.gameManager` _returnvalue))

(event `self.StaticMeshComponent.OnBeginCursorOver`
  (params (TouchedComponent :type "PrimitiveComponent Object Reference"))
  (`PrimitiveComponent.SetRenderCustomDepth` (`self.StaticMeshComponent`) true))

(event `self.StaticMeshComponent.OnEndCursorOver`
  (params (TouchedComponent :type "PrimitiveComponent Object Reference"))
  (if (not (`self.interacted`))
    (`PrimitiveComponent.SetRenderCustomDepth` (`self.StaticMeshComponent`) false)))

(event `self.StaticMeshComponent.OnClicked`
  (params (TouchedComponent :type "PrimitiveComponent Object Reference") (ButtonPressed :type "Key Structure"))
  (bind _playerref (`/Game/Blueprints/BP_GameManager.playerRef` (`self.gameManager`)))
  (bind _charactermovement (`Character.CharacterMovement` _playerref))
  (if (and (<= (`self.GetDistanceTo` _playerref self) (`/Game/TopDown/Blueprints/BP_TopDownCharacter.interactDistance` _playerref)) (`|EnumInequality` (`CharacterMovementComponent.MovementMode` _charactermovement) "MOVE_None") (not (`self.interacted`)))
    (`CharacterMovementComponent.SetMovementMode` _charactermovement "MOVE_None" 0)
    (`KismetSystemLibrary.PrintString` "interacted")
    (set `self.interacted` true)
    (`PrimitiveComponent.SetRenderCustomDepth` (`self.StaticMeshComponent`) true)
    (bind _returnvalue (`|CreateWidget` "/Game/Blueprints/UI/WB_Destructable.WB_Destructable_C"))
    (`UserWidget.AddToViewport` _returnvalue 0)
    (`/Game/Blueprints/UI/WB_Destructable.InitDestructableWB` _returnvalue self)))

(fn `UserConstructionScript`)